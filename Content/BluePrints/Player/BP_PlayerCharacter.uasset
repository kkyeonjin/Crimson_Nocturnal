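; Player character Blueprint that wires up its blade, kick and raycast components when play begins.
; BeginPlay passes left and right trace points and blade boxes to Blade, and leg trace points and the kick collision to Kick.
; It also hands the capsule component to Raycast.
; The Blueprint holds only this setup, as overlap, tick and construction script are empty.
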(event `self.ReceiveBeginPlay`
  (`WeaponComponent.InitializeWeaponComponents` (`self.Blade`) (`self.TraceStart_L`) (`self.TraceEnd_L`) (`self.TraceStart_R`) (`self.TraceEnd_R`) (`self.Blade_L`) (`self.Blade_R`))
  (`KickComponent.InitializeKickComponents` (`self.Kick`) (`self.TraceStart`) (`self.TraceEnd`) (`self.KickCollision`))
  (`RaycastComponent.InitializeCapsuleCollision` (`self.Raycast`) (`self.CapsuleComponent`)))

(fn `UserConstructionScript`)